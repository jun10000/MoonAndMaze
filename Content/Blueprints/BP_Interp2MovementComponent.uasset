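; BP_Interp2MovementComponent is an actor component that moves its owner back and forth along a direction with sine-wave motion.
; BeginPlay caches the owner's starting location.
; Each tick it sets the owner's position with sweep to that origin plus the normalized MoveDirection, scaled by MoveDistance and a sine of the owner's lifetime times SineSpeedDegree.
; Deriving position from elapsed time avoids accumulated drift.
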(event `self.ReceiveBeginPlay`
  (set `self.OriginalLocation` (`Actor.K2_GetActorLocation` (`self.GetOwner`))))

(event `self.ReceiveTick`
  (params (DeltaSeconds :type "Float (single-precision)"))
  (bind _returnvalue (`self.GetOwner`))
  (`Actor.K2_SetActorLocation` _returnvalue (+ (`self.OriginalLocation`) (* (`KismetMathLibrary.DegSin` (* (`Actor.GetGameTimeSinceCreation` _returnvalue) (`self.SineSpeedDegree`))) (`self.MoveDistance`) (`KismetMathLibrary.Normal` (`self.MoveDirection`)))) true false))