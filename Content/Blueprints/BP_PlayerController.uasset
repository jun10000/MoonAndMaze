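; Player controller that maps Enhanced Input actions to pawn movement, camera look, pausing and quitting.
; BeginPlay adds the default mapping context.
; Move input drives the pawn along the camera's forward and right vectors flattened to the horizontal plane, and look input adds yaw and inverted pitch.
; Pause is delegated to the game mode, while exit quits the game directly.
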(event `self.ReceiveBeginPlay`
  (`EnhancedInputSubsystemInterface.AddMappingContext` (subsystem `EnhancedInputLocalPlayerSubsystem`) "/Game/Input/IM_Default.IM_Default" 0 (struct)))

(event `EnhancedInput|/Game/Input/IA_Move`
  (params (ActionValue :type "Vector2D Structure") (ElapsedSeconds :type "Float (double-precision)") (TriggeredSeconds :type "Float (double-precision)") (InputAction :type "InputAction Object Reference" :default "/Game/Input/IA_Move.IA_Move"))
  (bind _returnvalue (`/Game/Blueprints/BP_FunctionLibrary.GetMyPlayerPawn`))
  (bind (_x _y) (`KismetMathLibrary.BreakVector2D` ActionValue))
  (bind _camera (`/Game/Blueprints/BP_PlayerPawn.Camera` _returnvalue))
  (:`Triggered`
    (`Pawn.AddMovementInput` _returnvalue (`KismetMathLibrary.Vector_Normal2D` (`SceneComponent.GetForwardVector` _camera)) _y false)
    (`Pawn.AddMovementInput` _returnvalue (`KismetMathLibrary.Vector_Normal2D` (`SceneComponent.GetRightVector` _camera)) _x false)))

(event `EnhancedInput|/Game/Input/IA_Exit`
  (params (ActionValue :type Boolean) (ElapsedSeconds :type "Float (double-precision)") (TriggeredSeconds :type "Float (double-precision)") (InputAction :type "InputAction Object Reference" :default "/Game/Input/IA_Exit.IA_Exit"))
  (:`Started`
    (`KismetSystemLibrary.QuitGame` null "Quit")))

(event `EnhancedInput|/Game/Input/IA_Pause`
  (params (ActionValue :type Boolean) (ElapsedSeconds :type "Float (double-precision)") (TriggeredSeconds :type "Float (double-precision)") (InputAction :type "InputAction Object Reference" :default "/Game/Input/IA_Pause.IA_Pause"))
  (:`Started`
    (`/Game/Blueprints/BP_GameMode.SwitchPause` (`/Game/Blueprints/BP_FunctionLibrary.GetMyGameMode`))))

(event `EnhancedInput|/Game/Input/IA_MoveCameraAngle`
  (params (ActionValue :type "Vector2D Structure") (ElapsedSeconds :type "Float (double-precision)") (TriggeredSeconds :type "Float (double-precision)") (InputAction :type "InputAction Object Reference" :default "/Game/Input/IA_MoveCameraAngle.IA_MoveCameraAngle"))
  (:`Triggered`
    (`self.AddYawInput` ActionValue_X)
    (`self.AddPitchInput` (* ActionValue_Y -1.0))))

(fn `UserConstructionScript`)