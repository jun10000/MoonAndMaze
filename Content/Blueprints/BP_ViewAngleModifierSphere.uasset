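; View angle modifier sphere actor that computes how strongly its effect applies, based on the player pawn's distance from it.
; The construction script caps the max-effect radius at the enabling radius and sizes the inner and outer spheres to match.
; GetCurrentEffectRatio returns 1 within the inner radius, falling linearly to 0 at the outer one.
; The ratio uses clamped distance rather than overlap events; applying it to the view happens outside these graphs.
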(fn `GetCurrentEffectRatio`
  (returns (ReturnValue :type "Float (double-precision)"))
  (bind _effectenablingradius (`self.EffectEnablingRadius`))
  (bind _effectmaxradius (`self.EffectMaxRadius`))
  (bind _returnvalue (- (`KismetMathLibrary.FClamp` (`KismetMathLibrary.Vector_Distance` (`self.K2_GetActorLocation`) (`self.K2_GetActorLocation` (`/Game/Blueprints/BP_FunctionLibrary.GetMyPlayerPawn`))) 0.0 _effectenablingradius) _effectmaxradius))
  (return (- 1.0 (`KismetMathLibrary.SafeDivide` (`KismetMathLibrary.SelectFloat` _returnvalue 0.0 (>= _returnvalue 0.0)) (- _effectenablingradius _effectmaxradius)))))

(fn `UserConstructionScript`
  (bind _effectenablingradius (`self.EffectEnablingRadius`))
  (`parent.UserConstructionScript`)
  (if (> (`self.EffectMaxRadius`) _effectenablingradius)
    (set `self.EffectMaxRadius` _effectenablingradius))
  (`SphereComponent.SetSphereRadius` (`self.SphereOuter`) (`self.EffectEnablingRadius`) true)
  (`SphereComponent.SetSphereRadius` (`self.SphereInner`) (`self.EffectMaxRadius`) true))