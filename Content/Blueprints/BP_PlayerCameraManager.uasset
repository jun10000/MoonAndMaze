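; Player camera manager that drives the camera's pitch, yaw and roll limits from a list of view angle modifiers.
; Each tick it applies the blended limits: the original angles with no modifiers, a lerp toward a single modifier by its effect ratio.
; With several, it lerps successively through them, weighting each by its share of the summed effect ratios.
; It also exposes forward, right and up vectors of the camera rotation.
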(event `self.ReceiveTick`
  (params (DeltaSeconds :type "Float (single-precision)"))
  (bind (_viewanglemin _viewanglemax) (`self.GetCurrentViewAngle`))
  (set `self.ViewRollMin` (.roll _viewanglemin))
  (set `self.ViewPitchMin` (.pitch _viewanglemin))
  (set `self.ViewYawMin` (.yaw _viewanglemin))
  (set `self.ViewRollMax` (.roll _viewanglemax))
  (set `self.ViewPitchMax` (.pitch _viewanglemax))
  (set `self.ViewYawMax` (.yaw _viewanglemax)))

(fn `GetCameraForwardVector`
  (returns (ReturnValue :type "Vector Structure"))
  (return (`KismetMathLibrary.GetForwardVector` (`self.GetCameraRotation`))))

(fn `GetCameraRightVector`
  (returns (ReturnValue :type "Vector Structure"))
  (return (`KismetMathLibrary.GetRightVector` (`self.GetCameraRotation`))))

(fn `GetCameraUpVector`
  (returns (ReturnValue :type "Vector Structure"))
  (return (`KismetMathLibrary.GetUpVector` (`self.GetCameraRotation`))))

(fn `GetCurrentViewAngle`
  (returns (ViewAngleMin :type "Rotator Structure") (ViewAngleMax :type "Rotator Structure"))
  (locals (ResultMin :type "Rotator Structure" :default (struct)) (ResultMax :type "Rotator Structure" :default (struct)) (EffectRatioSum :type "Float (double-precision)"))
  (bind _viewanglemodifiers (`self.ViewAngleModifiers`))
  (bind _output (`|GetArrayItem` (`self.ViewAngleModifiers`)))
  (bind _output_2 (`|GetArrayItem` _viewanglemodifiers))
  (bind _returnvalue (`/Game/Blueprints/BP_ViewAngleModifierSphere.GetCurrentEffectRatio` _output))
  (switch `int` (`KismetArrayLibrary.Array_Length` (`self.ViewAngleModifiers`))
    (:`Default`
      (set `local.ResultMin` (`/Game/Blueprints/BP_ViewAngleModifierSphere.ViewAngleMin` _output_2))
      (set `local.ResultMax` (`/Game/Blueprints/BP_ViewAngleModifierSphere.ViewAngleMax` _output_2))
      (for _array_element _viewanglemodifiers
        (set `local.EffectRatioSum` (+ (`local.EffectRatioSum`) (`/Game/Blueprints/BP_ViewAngleModifierSphere.GetCurrentEffectRatio` _array_element))))
      (for _array_element_2 _viewanglemodifiers
        (bind _returnvalue_2 (`KismetMathLibrary.SafeDivide` (`/Game/Blueprints/BP_ViewAngleModifierSphere.GetCurrentEffectRatio` _array_element_2) (`local.EffectRatioSum`)))
        (set `local.ResultMin` (`KismetMathLibrary.RLerp` (`local.ResultMin`) (`/Game/Blueprints/BP_ViewAngleModifierSphere.ViewAngleMin` _array_element_2) _returnvalue_2))
        (set `local.ResultMax` (`KismetMathLibrary.RLerp` (`local.ResultMax`) (`/Game/Blueprints/BP_ViewAngleModifierSphere.ViewAngleMax` _array_element_2) _returnvalue_2)))
      (return (`local.ResultMin`) (`local.ResultMax`)))
    (:`0`
      (return (`self.OriginalViewAngleMin`) (`self.OriginalViewAngleMax`)))
    (:`1`
      (return (`KismetMathLibrary.RLerp` (`self.OriginalViewAngleMin`) (`/Game/Blueprints/BP_ViewAngleModifierSphere.ViewAngleMin` _output) _returnvalue) (`KismetMathLibrary.RLerp` (`self.OriginalViewAngleMax`) (`/Game/Blueprints/BP_ViewAngleModifierSphere.ViewAngleMax` _output) _returnvalue)))))

(fn `UserConstructionScript`)