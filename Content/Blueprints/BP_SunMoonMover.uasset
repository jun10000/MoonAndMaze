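; BP_SunMoonMover is an actor that animates a referenced directional light's pitch, presumably to move the sun or moon.
; BeginPlay sets the actor's own rotation to the start pitch, borrowing the light's roll and yaw.
; Tick raises the light's pitch at a frame-rate-independent speed, preserving roll and yaw.
; On reaching the end pitch, it clamps the rotation, disables its tick and fires OnPitchReachesEnd.
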(event `self.ReceiveBeginPlay`
  (bind (_returnvalue_roll _returnvalue_pitch _returnvalue_yaw) (`KismetMathLibrary.BreakRotator` (`self.K2_GetActorRotation` (`self.DirectionalLight`))))
  (`self.K2_SetActorRotation` (`KismetMathLibrary.MakeRotator` _returnvalue_roll (`self.PitchStart`) _returnvalue_yaw)))

(event `self.ReceiveTick`
  (params (DeltaSeconds :type "Float (single-precision)"))
  (bind _pitchend (`self.PitchEnd`))
  (bind _directionallight (`self.DirectionalLight`))
  (bind (_returnvalue_roll _returnvalue_pitch _returnvalue_yaw) (`KismetMathLibrary.BreakRotator` (`self.K2_GetActorRotation` (`self.DirectionalLight`))))
  (bind _returnvalue (+ (* (`self.PitchDelta`) DeltaSeconds) _returnvalue_pitch))
  (if (>= _returnvalue _pitchend)
    (`self.K2_SetActorRotation` _directionallight (`KismetMathLibrary.MakeRotator` _returnvalue_roll _pitchend _returnvalue_yaw) false)
    (`self.SetActorTickEnabled` false)
    (`self.OnPitchReachesEnd`)
    (else
      (`self.K2_SetActorRotation` _directionallight (`KismetMathLibrary.MakeRotator` _returnvalue_roll _returnvalue _returnvalue_yaw) false))))

(fn `UserConstructionScript`)