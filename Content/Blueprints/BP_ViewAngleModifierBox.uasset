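; Box-shaped view angle modifier volume that computes effect strength from the player pawn's position.
; Construction sizes an outer enabling box and an inner full-effect box, capping inner extents to outer and matching them on disabled axes.
; The ratio fades from 1 to 0 between boxes, using component line traces toward the center to find both boundaries along the player's direction.
; Only enabled axes count; with none, the ratio is 1.
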(fn `GetCurrentEffectRatio`
  (returns (ReturnValue :type "Float (double-precision)"))
  (locals (OriginLocation :type "Vector Structure" :default (0.0 0.0 0.0)) (TraceStartLocation :type "Vector Structure") (RawPlayerDistance :type "Float (double-precision)" :default 0.0) (InnerDistance :type "Float (double-precision)" :default 0.0) (OuterDistance :type "Float (double-precision)" :default 0.0))
  (bind (_returnvalue_x _returnvalue_y _returnvalue_z) (`KismetMathLibrary.BreakVector` (- (`self.K2_GetActorLocation` (`/Game/Blueprints/BP_FunctionLibrary.GetMyPlayerPawn`)) (`local.OriginLocation`))))
  (bind _returnvalue (`KismetMathLibrary.MakeVector` (`KismetMathLibrary.SelectFloat` _returnvalue_x 0.0 (`self.IsAxisXEnable`)) (`KismetMathLibrary.SelectFloat` _returnvalue_y 0.0 (`self.IsAxisYEnable`)) (`KismetMathLibrary.SelectFloat` _returnvalue_z 0.0 (`self.IsAxisZEnable`))))
  (if (or (`self.IsAxisXEnable`) (`self.IsAxisYEnable`) (`self.IsAxisZEnable`))
    (`|ExecutionSequence`
      (:`then_0`
        (set `local.OriginLocation` (`self.K2_GetActorLocation`))
        (set `local.RawPlayerDistance` (`KismetMathLibrary.VSize` _returnvalue))
        (set `local.TraceStartLocation` (+ (* (`KismetMathLibrary.Normal` _returnvalue) (`self.GetTraceLength`)) (`local.OriginLocation`))))
      (:`then_1`
        (bind (_hitlocation _hitnormal _bonename _outhit _returnvalue_2) (`PrimitiveComponent.K2_LineTraceComponent` (`self.BoxInner`) (`local.TraceStartLocation`) (`local.OriginLocation`) false false false))
        (if _returnvalue_2
          (set `local.InnerDistance` (`KismetMathLibrary.Vector_Distance` (`local.OriginLocation`) _hitlocation))
          (else
            (`/Game/Blueprints/BP_FunctionLibrary.PrintError` self "Could not get InnerDistance"))))
      (:`then_2`
        (bind (_hitlocation_2 _hitnormal_2 _bonename_2 _outhit_2 _returnvalue_3) (`PrimitiveComponent.K2_LineTraceComponent` (`self.BoxOuter`) (`local.TraceStartLocation`) (`local.OriginLocation`) false false false))
        (if _returnvalue_3
          (set `local.OuterDistance` (`KismetMathLibrary.Vector_Distance` (`local.OriginLocation`) _hitlocation_2))
          (else
            (`/Game/Blueprints/BP_FunctionLibrary.PrintError` self "Could not get OuterDistance"))))
      (:`then_3`
        (return (- 1.0 (`KismetMathLibrary.FClamp` (`KismetMathLibrary.NormalizeToRange` (`KismetMathLibrary.FClamp` (`local.RawPlayerDistance`) 0.0 (`local.OuterDistance`)) (`local.InnerDistance`) (`local.OuterDistance`)))))))
    (else
      (return 1.0))))

(fn `GetTraceLength`
  (returns (ReturnValue :type "Float (double-precision)"))
  (bind (_returnvalue_x _returnvalue_y _returnvalue_z) (`KismetMathLibrary.BreakVector` (* (`BoxComponent.BoxExtent` (`self.BoxOuter`)) 2.0)))
  (return (`KismetMathLibrary.Sqrt` (+ (+ (`KismetMathLibrary.MultiplyMultiply_FloatFloat` _returnvalue_x 2.0) (`KismetMathLibrary.MultiplyMultiply_FloatFloat` _returnvalue_y 2.0)) (`KismetMathLibrary.MultiplyMultiply_FloatFloat` _returnvalue_z 2.0)))))

(fn `UserConstructionScript`
  (bind (_effectmaxextent_x _effectmaxextent_y _effectmaxextent_z) (`KismetMathLibrary.BreakVector` (`self.EffectMaxExtent`)))
  (bind (_effectenablingextent_x _effectenablingextent_y _effectenablingextent_z) (`KismetMathLibrary.BreakVector` (`self.EffectEnablingExtent`)))
  (`parent.UserConstructionScript`)
  (set `self.EffectMaxExtent` (`KismetMathLibrary.MakeVector` (`KismetMathLibrary.SelectFloat` _effectenablingextent_x _effectmaxextent_x (or (> _effectmaxextent_x _effectenablingextent_x) (not (`self.IsAxisXEnable`)))) (`KismetMathLibrary.SelectFloat` _effectenablingextent_y _effectmaxextent_y (or (> _effectmaxextent_y _effectenablingextent_y) (not (`self.IsAxisYEnable`)))) (`KismetMathLibrary.SelectFloat` _effectenablingextent_z _effectmaxextent_z (or (> _effectmaxextent_z _effectenablingextent_z) (not (`self.IsAxisZEnable`))))))
  (`BoxComponent.SetBoxExtent` (`self.BoxOuter`) (`self.EffectEnablingExtent`) true)
  (`BoxComponent.SetBoxExtent` (`self.BoxInner`) (`self.EffectMaxExtent`) true))