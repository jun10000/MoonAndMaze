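; Blueprint function library of global shortcuts to the game's own game mode, player controller and pawn classes, plus on-screen logging and UI helpers.
; The getters cast the engine's game mode and player index 0 objects, while error and warning helpers print colored, prefixed strings.
; ShowWidget and HideWidget forward a widget class to the game mode's WidgetManager, picking the input mode by whether that class implements I_WidgetOperatable.
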(fn `GetMyGameMode`
  (returns (ReturnValue :type "/Game/Blueprints/BP_GameMode Object Reference"))
  (return (cast `/Game/Blueprints/BP_GameMode` (`GameplayStatics.GetGameMode` null) :!pure true)))

(fn `GetMyPlayerController`
  (returns (ReturnValue :type "/Game/Blueprints/BP_PlayerController Object Reference"))
  (return (cast `/Game/Blueprints/BP_PlayerController` (`GameplayStatics.GetPlayerController` null) :!pure true)))

(fn `GetMyPlayerPawn`
  (returns (ReturnValue :type "/Game/Blueprints/BP_PlayerPawn Object Reference"))
  (return (cast `/Game/Blueprints/BP_PlayerPawn` (`GameplayStatics.GetPlayerPawn` null) :!pure true)))

(fn `GetWidgetManager`
  (returns (ReturnValue :type "/Game/Blueprints/BP_WidgetManagerComponent Object Reference"))
  (return (`/Game/Blueprints/BP_GameMode.WidgetManager` (`self.GetMyGameMode` null))))

(fn `HideWidget`
  (params (WidgetClass :type "UserWidget Class Reference"))
  (`/Game/Blueprints/BP_WidgetManagerComponent.HideWidget` (`self.GetWidgetManager` null) (make `/Game/Blueprints/Struct/ST_WidgetKey` WidgetClass) null (select `bool` (`KismetSystemLibrary.DoesClassImplementInterface` WidgetClass "/Game/Blueprints/Interface/I_WidgetOperatable.I_WidgetOperatable_C") :`false` "NewEnumerator0" :`true` "NewEnumerator1" :!type "/Game/Blueprints/Enum/E_ChangeControllerInputMode Enum")))

(fn `PrintError`
  (params (WorldContextObject :type "Object Object Reference") (Message :type String) (Duration :type "Float (single-precision)" :default 10.0))
  (`KismetSystemLibrary.PrintString` WorldContextObject (`KismetStringLibrary.Concat_StrStr` "Error: " Message) true true (struct :`R` 1.0 :`A` 1.0) Duration))

(fn `PrintWarning`
  (params (WorldContextObject :type "Object Object Reference") (Message :type String) (PrintToScreen :type Boolean) (Duration :type "Float (single-precision)" :default 10.0))
  (`KismetSystemLibrary.PrintString` WorldContextObject (`KismetStringLibrary.Concat_StrStr` "Warning: " Message) PrintToScreen true (struct :`R` 1.0 :`G` 0.5 :`A` 1.0) Duration))

(fn `ShowWidget`
  (params (WidgetClass :type "UserWidget Class Reference"))
  (`/Game/Blueprints/BP_WidgetManagerComponent.ShowWidget` (`self.GetWidgetManager` null) (make `/Game/Blueprints/Struct/ST_WidgetKey` WidgetClass) null (select `bool` (`KismetSystemLibrary.DoesClassImplementInterface` WidgetClass "/Game/Blueprints/Interface/I_WidgetOperatable.I_WidgetOperatable_C") :`false` "NewEnumerator0" :`true` "NewEnumerator3" :!type "/Game/Blueprints/Enum/E_ChangeControllerInputMode Enum")))