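; Player pawn with health, an item inventory, an area attack and respawn on death.
; A state switch lets damage land only in Normal, followed by timed invincibility or, at zero HP, death.
; Death disables movement and destroys the pawn after a delay; EndPlay then spawns and possesses a replacement at the player start.
; Attack destroys spawner-tracked actors within a cylinder around the pawn, and Tick clamps camera arm length.
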(event `self.ReceiveBeginPlay`
  (set `self.HP` (`self.MaxHP`))
  (`KismetSystemLibrary.Delay` (`self.InvincibleDuration`))
  (set `self.State` "NewEnumerator0"))

(event `self.ReceiveAnyDamage`
  (params (Damage :type "Float (single-precision)") (DamageType :type "DamageType Object Reference") (InstigatedBy :type "Controller Object Reference") (DamageCauser :type "Actor Object Reference"))
  (switch `/Game/Blueprints/Enum/E_PlayerState` (`self.State`)
    (:`NewEnumerator0`
      (bind _output_get (set `self.HP` (- (`self.HP`) Damage)))
      (if (> _output_get 0.0)
        (set `self.State` "NewEnumerator1")
        (`KismetSystemLibrary.Delay` (`self.InvincibleDuration`))
        (set `self.State` "NewEnumerator0")
        (else
          (set `self.State` "NewEnumerator2")
          (`self.Event_Die`))))))

(event `Event_Die`
  (`CharacterMovementComponent.DisableMovement` (`self.CharacterMovement`))
  (`KismetSystemLibrary.Delay` (`self.DyingDuration`))
  (`self.K2_DestroyActor`))

(event `self.ReceiveEndPlay`
  (params (EndPlayReason :type "EEndPlayReason Enum" :default "Destroyed"))
  (switch `EEndPlayReason` EndPlayReason
    (:`Destroyed`
      (bind _returnvalue (`|SpawnActorFromClass` "BP_PlayerPawn_C" (`self.GetTransform` (`GameModeBase.K2_FindPlayerStart` (`/Game/Blueprints/BP_FunctionLibrary.GetMyGameMode`) (`/Game/Blueprints/BP_FunctionLibrary.GetMyPlayerController`) "")) "Undefined" "MultiplyWithRoot" null null))
      (`Controller.Possess` (`/Game/Blueprints/BP_FunctionLibrary.GetMyPlayerController`) _returnvalue))))

(event `self.ReceiveTick`
  (params (DeltaSeconds :type "Float (single-precision)"))
  (bind _springarm (`self.SpringArm`))
  (set `SpringArmComponent.TargetArmLength` (`KismetMathLibrary.FClamp` (`SpringArmComponent.TargetArmLength` _springarm) (`self.CurrentArmLengthMin`) (`self.CurrentArmLengthMax`)) _springarm))

(fn `AddItem`
  (params (Item :type "/Game/Blueprints/Enum/E_PlayerItem Enum" :default "NewEnumerator0") (Count :type Integer :default 1))
  (bind _items (`self.Items`))
  (`BlueprintMapLibrary.Map_Add` _items Item (+ (`BlueprintMapLibrary.Map_Find` _items Item) Count)))

(fn `Attack`
  (params (Item :type "/Game/Blueprints/Enum/E_PlayerItem Enum" :default "NewEnumerator0"))
  (locals (DestroyActors :type "Array of Actor Object Reference"))
  (bind _returnvalue (`self.K2_GetActorLocation`))
  (switch `/Game/Blueprints/Enum/E_PlayerItem` Item
    (:`NewEnumerator0`
      (for _array_element (`/Game/Blueprints/BP_SpawnerComponent.GetSpawnedActors` (`self.BP_SpawnerComponent`))
        (bind _returnvalue_2 (`self.K2_GetActorLocation` _array_element))
        (if (and (< (`KismetMathLibrary.Vector_Distance2D` _returnvalue_2 _returnvalue) (`self.AttackMoon_Radius`)) (< (`KismetMathLibrary.Abs` (- (.z _returnvalue_2) (.z _returnvalue))) (`self.AttackMoon_HalfHeight`)))
          (`KismetArrayLibrary.Array_Add` (`local.DestroyActors`) _array_element)))
      (for _array_element_2 (`local.DestroyActors`)
        (`self.K2_DestroyActor` _array_element_2)))))

(fn `GetItemNum`
  (params (Item :type "/Game/Blueprints/Enum/E_PlayerItem Enum" :default "NewEnumerator0"))
  (returns (ReturnValue :type Integer) (IsExist :type Boolean))
  (bind _value (`BlueprintMapLibrary.Map_Find` (`self.Items`) Item))
  (return _value (> _value 0)))

(fn `UserConstructionScript`)