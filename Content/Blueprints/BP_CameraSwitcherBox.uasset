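; BP_CameraSwitcherBox is a trigger actor that changes the player's camera view when BP_PlayerPawn enters it.
; On overlap it blends the view target to either itself or the pawn, depending on IsViewTargetPlayer, with configurable ease-in-out blend settings.
; The construction script sets the spring arm's length and pitch.
; Each tick the arm keeps that pitch while its relative yaw follows the player controller's control rotation.
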(event `self.ReceiveTick`
  (params (DeltaSeconds :type "Float (single-precision)"))
  (bind (_returnvalue_roll _returnvalue_pitch _returnvalue_yaw) (`KismetMathLibrary.BreakRotator` (`Controller.GetControlRotation` (`/Game/Blueprints/BP_FunctionLibrary.GetMyPlayerController`))))
  (`SceneComponent.K2_SetRelativeRotation` (`self.SpringArm`) (`KismetMathLibrary.MakeRotator` 0.0 (`self.CameraRotationPitch`) _returnvalue_yaw) false false))

(event `self.ReceiveActorBeginOverlap`
  (params (OtherActor :type "Actor Object Reference"))
  (bind _asbp_player_pawn (cast `/Game/Blueprints/BP_PlayerPawn` OtherActor))
  (`PlayerController.SetViewTargetWithBlend` (`/Game/Blueprints/BP_FunctionLibrary.GetMyPlayerController`) (select `bool` (`self.IsViewTargetPlayer`) :`false` self :`true` _asbp_player_pawn :!type "Actor Object Reference") (`self.CameraBlendTime`) "VTBlend_EaseInOut" (`self.CameraBlendExp`) false))

(fn `UserConstructionScript`
  (bind _springarm (`self.SpringArm`))
  (set `SpringArmComponent.TargetArmLength` (`self.CameraArmLength`) _springarm)
  (`SceneComponent.K2_SetRelativeRotation` _springarm (`KismetMathLibrary.MakeRotator` 0.0 (`self.CameraRotationPitch`)) false false))