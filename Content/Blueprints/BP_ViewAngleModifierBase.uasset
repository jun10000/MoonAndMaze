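; Base actor for zones that modify the camera view angle while the player pawn overlaps them.
; On begin overlap with BP_PlayerPawn it adds itself uniquely to the player camera manager's ViewAngleModifiers list, and removes itself on end overlap.
; GetCurrentEffectRatio is a stub returning zero, so this base supplies no effect strength of its own.
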(event `self.ReceiveActorBeginOverlap`
  (params (OtherActor :type "Actor Object Reference"))
  (bind _returnvalue (`/Game/Blueprints/BP_FunctionLibrary.GetMyPlayerCameraManager`))
  (cast `/Game/Blueprints/BP_PlayerPawn` OtherActor)
  (`/Engine/EditorBlueprintResources/StandardMacros.IsValid` _returnvalue
    (:`Is Valid`
      (`KismetArrayLibrary.Array_AddUnique` (`/Game/Blueprints/BP_PlayerCameraManager.ViewAngleModifiers` _returnvalue) self))))

(event `self.ReceiveActorEndOverlap`
  (params (OtherActor :type "Actor Object Reference"))
  (bind _returnvalue (`/Game/Blueprints/BP_FunctionLibrary.GetMyPlayerCameraManager`))
  (cast `/Game/Blueprints/BP_PlayerPawn` OtherActor)
  (`/Engine/EditorBlueprintResources/StandardMacros.IsValid` _returnvalue
    (:`Is Valid`
      (`KismetArrayLibrary.Array_RemoveItem` (`/Game/Blueprints/BP_PlayerCameraManager.ViewAngleModifiers` _returnvalue) self))))

(fn `GetCurrentEffectRatio`
  (returns (ReturnValue :type "Float (double-precision)"))
  (locals (OriginLocation :type "Vector Structure" :default (0.0 0.0 0.0)) (TraceEndLocation :type "Vector Structure") (RawPlayerDistance :type "Float (double-precision)" :default 0.0) (InnerDistance :type "Float (double-precision)" :default 0.0) (OuterDistance :type "Float (double-precision)" :default 0.0))
  (return 0.0))

(fn `UserConstructionScript`)