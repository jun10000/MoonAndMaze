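; BP_EnemySpawner is an enemy spawner actor that so far only finds and visualizes candidate spawn points in shadow, without spawning anything.
; SpawnEnemy picks a random navigable point within a radius of the actor, then line-traces from it against the directional light's forward vector.
; A blocking hit on the Visibility channel means the point is shaded from the light, so it gets a debug point.
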(event `SpawnEnemy`
  (bind (_randomlocation _returnvalue) (`NavigationSystemV1.K2_GetRandomLocationInNavigableRadius` (`self.K2_GetActorLocation`) (`self.NavigableRadius`) (`self.NavigationData`) null))
  (if _returnvalue
    (bind (_outhit _returnvalue_2) (`KismetSystemLibrary.LineTraceSingle` :`Start` _randomlocation :`End` (- _randomlocation (* (`self.GetActorForwardVector` (`self.DirectionalLight`)) (`self.TraceDistance`))) :`TraceChannel` "TraceTypeQuery1" :`DrawDebugType` "ForDuration"))
    (if _returnvalue_2
      (`KismetSystemLibrary.DrawDebugPoint` _randomlocation 15.0 (struct :`R` 1.0 :`G` 1.0 :`A` 1.0) 5.0))))

(fn `UserConstructionScript`)