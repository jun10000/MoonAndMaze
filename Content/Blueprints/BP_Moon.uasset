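; BP_Moon is a moon actor with a glowing sphere and a point light.
; The construction script creates a dynamic instance of M_Moon on the sphere and sets its emissive brightness and color parameters.
; It then applies the same color and a separate light brightness to the point light, keeping surface and light tint matched.
; The event graph holds only disabled placeholder events, so there is no runtime logic.
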(fn `UserConstructionScript`
  (bind _pointlight (`self.PointLight`))
  (`|ExecutionSequence`
    (:`then_0`
      (bind _returnvalue (`PrimitiveComponent.CreateDynamicMaterialInstance` (`self.Sphere`) 0 "/Game/Prop/Material/M_Moon.M_Moon" "None"))
      (`MaterialInstanceDynamic.SetScalarParameterValue` _returnvalue "Brightness" (`self.EmissiveBrightness`))
      (`MaterialInstanceDynamic.SetVectorParameterValue` _returnvalue "Color" (`self.Color`)))
    (:`then_1`
      (`LightComponent.SetIntensity` _pointlight (`self.LightBrightness`))
      (`LightComponent.SetLightColor` _pointlight (`self.Color`) false))))